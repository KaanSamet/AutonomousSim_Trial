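; BP_LIDAR_DataFiller rebuilds stored LIDAR scan data in the level as sprite actors behind a loading screen.
; On BeginPlay it reads impact points, rotations and the pawn location from BP_GameInstance.
; SpawnData places BP_PaperSpriteActors in SpawnRange-sized batches, yielding with zero-length delays and updating the widget's progress.
; When no full batch remains, it spawns and possesses SportsCar_Pawn and removes the loading screen.
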(event Custom|Spawn%20Data
  (bind _datafillloadingscreen (Variables|Default|GetDataFillLoadingScreen))
  (if (Utilities|Array|IsValidIndex (Variables|Default|GetUp%20LIDAR%20Impact%20Points) (+ (Variables|Default|GetSpawnRegulatorIndexer) (Variables|Default|GetSpawnRange))) :!label _label
    (Utilities|IsValid _datafillloadingscreen
      (:Is%20Valid
        (Default|RefreshLoadingScreenData _datafillloadingscreen (/ (Math|Conversions|ToFloat(Integer) (Variables|Default|GetSpawnRegulatorIndexer)) (Math|Conversions|ToFloat(Integer) (Utilities|Array|Length (Variables|Default|GetUp%20LIDAR%20Impact%20Points)))))
        (for _index (range (Variables|Default|GetSpawnRegulatorIndexer) (+ (Variables|Default|GetSpawnRegulatorIndexer) (Variables|Default|GetSpawnRange)))
          (Game|SpawnActorfromClass "/Game/Blueprints/BP_PaperSpriteActor.BP_PaperSpriteActor_C" (Math|Transform|MakeTransform (Utilities|Array|Get(acopy) (Variables|Default|GetUp%20LIDAR%20Impact%20Points) _index) (Utilities|Array|Get(acopy) (Variables|Default|GetUp%20LIDAR%20Impact%20Rotations) _index) "1.000000,1.000000,1.000000") "AdjustIfPossibleButDontSpawnIfColliding" "MultiplyWithRoot" 0 0))
        (Variables|Default|SetSpawnRegulatorIndexer (+ (Variables|Default|GetSpawnRegulatorIndexer) (Variables|Default|GetSpawnRange)))
        (Utilities|FlowControl|Delay 0.0)
        (goto _label)))
    (else
      (CallFunction|SpawnPawn)
      (Widget|RemovefromParent (Variables|Default|GetDataFillLoadingScreen)))))

(event Custom|SpawnPawn
  (bind _returnvalue (Game|SpawnActorfromClass "/Game/VehicleTemplate/Blueprints/SportsCar/SportsCar_Pawn.SportsCar_Pawn_C" (Math|Transform|MakeTransform (Variables|Default|GetPawn%20Location) "0, 0, 0" "1.000000,1.000000,1.000000") "AdjustIfPossibleButDontSpawnIfColliding" "MultiplyWithRoot" 0 0))
  (Pawn|Possess (Game|GetPlayerController 0) _returnvalue))

(event Custom|CreateLoadingScreenWidget
  (bind _returnvalue (UserInterface|CreateWidget "/Game/Blueprints/WBP_DataFillLoadingScreen.WBP_DataFillLoadingScreen_C" (Variables|Default|GetAs%20Vehicle%20Player%20Controller)))
  (bind _output_get (Variables|Default|SetDataFillLoadingScreen _returnvalue))
  (UserInterface|Viewport|AddtoViewport _output_get 0))

(event EventBeginPlay
  (bind _asbp_game_instance (Utilities|Casting|CastToBP_GameInstance (Game|GetGameInstance))
    (:then
      (Development|PrintString "GAMEINSTANCE CASTED" true true "(R=0.000000,G=0.660000,B=1.000000,A=1.000000)" 555.0)
      (Variables|Default|SetAs%20BP%20Game%20Instance _asbp_game_instance)
      (Variables|Default|SetPawn%20Location (Variables|/Game/Blueprints/Core/BP_GameInstance.BP_GameInstance_C|GetPawnLocation (Variables|Default|GetAs%20BP%20Game%20Instance)))
      (Variables|Default|SetUp%20LIDAR%20Impact%20Points (Variables|/Game/Blueprints/Core/BP_GameInstance.BP_GameInstance_C|GetUpLIDAR_ImpactPoints (Variables|Default|GetAs%20BP%20Game%20Instance)))
      (Variables|Default|SetUp%20LIDAR%20Impact%20Rotations (Variables|/Game/Blueprints/Core/BP_GameInstance.BP_GameInstance_C|GetUpLIDAR_ImpactRotations (Variables|Default|GetAs%20BP%20Game%20Instance)))
      (bind _asvehicle_player_controller (Utilities|Casting|CastToVehiclePlayerController (Game|GetPlayerController 0)))
      (Variables|Default|SetAs%20Vehicle%20Player%20Controller _asvehicle_player_controller)
      (CallFunction|CreateLoadingScreenWidget)
      (Utilities|FlowControl|Delay 0.0)
      (CallFunction|SpawnData))
    (:CastFailed
      (Development|PrintString "GAMEINSTANCE CAST FAILED" true true "(R=0.000000,G=0.660000,B=1.000000,A=1.000000)" 555.0))))

(event Collision|EventActorBeginOverlap
  (params (OtherActor :type Actor%20Object%20Reference)))

(event EventTick
  (params (DeltaSeconds :type Float%20%28single-precision%29)))

(fn ConstructionScript)