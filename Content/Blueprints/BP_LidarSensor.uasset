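; Simulated LiDAR sensor actor that scans its surroundings with Visibility line traces at a rate set by SensorHz via tick interval.
; Each tick loops through a full raster sweep, stepping the actor's own yaw and pitch and tracing along DirectionSpecifier, then zeroes its pitch and yaw.
; Blocking hits append to impact point and normal-derived rotation arrays, which are never cleared here; their sizes print as debug text.
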(event Custom|CustomEvent)

(event Custom|SpawnHitResults
  (params (LIDAR%20Hit%20Result :type Hit%20Result%20Structure) (BlockingHit :type Boolean))
  (bind (_bblockinghit _binitialoverlap _time _distance _location _impactpoint _normal _impactnormal) (Collision|BreakHitResult LIDAR%20Hit%20Result))
  (if BlockingHit
    (Utilities|Array|Add (Variables|Default|GetImpactPoints) (Math|Vector|MakeVector (.x _impactpoint) (.y _impactpoint) (.z _impactpoint)))
    (Utilities|Array|Add (Variables|Default|GetImpactRotations) (Math|Rotator|MakeRotfromY _impactnormal))))

(event EventBeginPlay
  (Actor|Tick|SetActorTickInterval (/ 1.0 (Variables|Exposed|GetSensorHz))))

(event EventTick
  (params (DeltaSeconds :type Float%20%28single-precision%29))
  (bind _returnvalue (Transformation|GetActorLocation))
  (bind _returnvalue_2 (Transformation|GetActorRotation))
  (Utilities|FlowControl|Sequence
    (:then_0
      (if (Variables|Default|GetTickCanFlow)
        (bind _output_get (Variables|Default|SetDelta%20Rotation%20Y%20%28Pitch%29 (* (Variables|Exposed|GetVerticalAngleOffset) -1.0)))
        (Class|Actor|AddActorWorldRotation (Math|Rotator|MakeRotator 0.0 _output_get 0.0))
        (bind (_outhit _returnvalue_3) (Collision|LineTraceByChannel _returnvalue (+ _returnvalue (* (Math|Vector|GetForwardVector (Variables|Default|GetDirectionSpecifier)) (Variables|Exposed|GetTraceLength))) "TraceTypeQuery1" false (Utilities|Array|MakeArray (Components|GetOwner)) "ForOneFrame" true (Variables|Default|GetTrace%20Color) "(R=0.000000,G=1.000000,B=0.000000,A=1.000000)" 0.25 :!label _label))
        (CallFunction|SpawnHitResults _outhit _returnvalue_3)
        (if (and (<= (Variables|Default|GetDelta%20Rotation%20Y%20%28Pitch%29) (Variables|Exposed|GetVerticalAngleOffset)) (>= (Variables|Default|GetDelta%20Rotation%20Y%20%28Pitch%29) (* (Variables|Exposed|GetVerticalAngleOffset) -1.0)))
          (if (< (Variables|Default|GetDelta%20Rotation%20Z%20%28Yaw%29) (Variables|Exposed|GetHorizontalAngleOffset))
            (Variables|Default|SetDelta%20Rotation%20Z%20%28Yaw%29 (+ (Variables|Default|GetDelta%20Rotation%20Z%20%28Yaw%29) (Variables|Exposed|GetTickStepHorizontal)))
            (Class|Actor|AddActorWorldRotation (Math|Rotator|MakeRotator 0.0 0.0 (Variables|Exposed|GetTickStepHorizontal)))
            (Variables|Default|SetTickCanFlow false :!label _label_2)
            (goto _label)
            (elif (== (Variables|Exposed|GetTickStepVertical) 0.0)
              (Variables|Default|SetTickCanFlow false)
              (Development|PrintString (Utilities|String|Append (Utilities|GetDisplayName self) " Tick Step Zero!"))
              (else
                (Variables|Default|SetDelta%20Rotation%20Y%20%28Pitch%29 (+ (Variables|Default|GetDelta%20Rotation%20Y%20%28Pitch%29) (Variables|Exposed|GetTickStepVertical)))
                (Variables|Default|SetDelta%20Rotation%20Z%20%28Yaw%29 0.0)
                (Class|Actor|AddActorWorldRotation (Math|Rotator|MakeRotator 0.0 (Variables|Exposed|GetTickStepVertical) 0.0))
                (goto _label_2)))))
        (Variables|Default|SetDelta%20Rotation%20Z%20%28Yaw%29 0.0)
        (Variables|Default|SetDelta%20Rotation%20Y%20%28Pitch%29 (* (Variables|Exposed|GetVerticalAngleOffset) -1.0))
        (Variables|Default|SetTickCanFlow true)
        (Class|Actor|AddActorWorldRotation (Math|Rotator|MakeRotator 0.0 (* (.pitch _returnvalue_2) -1.0) (* (.yaw _returnvalue_2) -1.0)))))
    (:then_1
      (Development|PrintString (Utilities|String|Append "IP: " (Utilities|String|ToString(Integer) (Utilities|Array|Length (Variables|Default|GetImpactPoints)))) true true "(R=0.000000,G=0.660000,B=1.000000,A=1.000000)" 0.1)
      (Development|PrintString (Utilities|String|Append "IR: " (Utilities|String|ToString(Integer) (Utilities|Array|Length (Variables|Default|GetImpactRotations)))) true true "(R=0.000000,G=0.660000,B=1.000000,A=1.000000)" 0.1))))

(fn ConstructionScript)