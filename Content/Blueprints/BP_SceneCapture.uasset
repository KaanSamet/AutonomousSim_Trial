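; BP_SceneCapture is a scene capture actor that saves what its 2D capture component renders as a numbered sequence of PNG files.
; BeginPlay starts an endless Delay loop that calls Export2DRenderTarget four times a second.
; Each export sets the render target's gamma, increments a counter for the file name, and writes the target to a PNGS folder in the project's Saved directory.
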(event Custom|Export2DRenderTarget
  (bind _capturecomponent2d (Variables|DecalActor|GetCaptureComponent2D))
  (bind _texturetarget (Variables|/Script/Engine.SceneCaptureComponent2D|GetTextureTarget _capturecomponent2d))
  (Variables|/Script/Engine.TextureRenderTarget|SetTargetGamma _texturetarget 2.0)
  (bind _result (Math|Integer|IncrementInt (Variables|Default|Getpngcounter))
    (:%20%20
      (Rendering|ExportRenderTarget _texturetarget (Utilities|String|Append (Class|KismetSystemLibrary|GetProjectSavedDirectory) "/PNGS") (Utilities|String|Append "pngtrial" (Utilities|String|ToString(Integer) _result) ".png")))))

(event EventBeginPlay
  (Utilities|FlowControl|Delay 0.25 :!label _label)
  (CallFunction|Export2DRenderTarget)
  (goto _label))

(event EventTick
  (params (DeltaSeconds :type Float%20%28single-precision%29)))

(fn ConstructionScript)